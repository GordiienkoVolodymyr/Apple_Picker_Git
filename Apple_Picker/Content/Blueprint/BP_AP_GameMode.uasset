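; BP_AP_GameMode is a game mode Blueprint with a game-over hook that receives whether the game was won.
; HandleGameOver only forwards that result to the parent implementation; BeginPlay, Tick and the construction script are empty.
; Disconnected nodes hold unused UI logic for a user widget and a delayed win/lose text on a game-over widget, with a comment noting a C++ implementation.
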(event EventBeginPlay)

(event EventTick
  (params (DeltaSeconds :type Float%20%28single-precision%29)))

(event EventHandleGameOver
  (params (Game_Won :type Boolean))
  (|CallParentFunction Game_Won))

(fn ConstructionScript)